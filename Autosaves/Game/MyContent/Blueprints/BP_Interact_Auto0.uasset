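; Interactable sign actor that shows a widget when something enters its sphere and lets the player toggle the sign text.
; Sphere overlap events, unfiltered by actor, set PlayerInRange and widget visibility, hiding both widget and text on exit.
; Input is enabled at BeginPlay, and Interact flips SignTextBorder visibility through a FlipFlop while in range.
; The FlipFlop does not reset on exit, and SetSignText is an empty stub.
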(event `self.ReceiveBeginPlay`
  ; //Allows user input when in collision sphere
  (`self.EnableInput` (`GameplayStatics.GetPlayerController` 0)))

(event `self.Sphere.OnComponentBeginOverlap`
  (params (OverlappedComponent :type "PrimitiveComponent Object Reference") (OtherActor :type "Actor Object Reference") (OtherComp :type "PrimitiveComponent Object Reference") (OtherBodyIndex :type Integer) (bFromSweep :type Boolean) (SweepResult :type "HitResult Structure (by ref)"))
  ; //When player enters/exits collision sphere will trigger  widget visibility
  ; //Sets player 'InRange' allowing text toggle
  (`SceneComponent.SetVisibility` (`self.Widget`) true false)
  (set `self.bPlayerInRange` true))

(event `self.Sphere.OnComponentEndOverlap`
  (params (OverlappedComponent :type "PrimitiveComponent Object Reference") (OtherActor :type "Actor Object Reference") (OtherComp :type "PrimitiveComponent Object Reference") (OtherBodyIndex :type Integer))
  ; //When player enters/exits collision sphere will trigger  widget visibility
  ; //Sets player 'InRange' allowing text toggle
  (`SceneComponent.SetVisibility` (`self.Widget`) false false)
  (`SceneComponent.SetVisibility` (`self.SignTextBorder`) false false)
  (set `self.bPlayerInRange` false))

(event `InputAction|Interact`
  (params (Key :type "Key Structure"))
  (bind _signtextborder (`self.SignTextBorder`))
  ; //Checks if player is in range
  ; //Waits for user input
  ; //Toggles visibility of widget when pressing e
  (:`Pressed`
    (if (`self.bPlayerInRange`)
      (`/Engine/EditorBlueprintResources/StandardMacros.FlipFlop`
        (:`A`
          (`SceneComponent.SetVisibility` _signtextborder true false))
        (:`B`
          (`SceneComponent.SetVisibility` _signtextborder false false))))))

(fn `setSignText`
  (params (NewText :type Text)))

(fn `UserConstructionScript`)