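; BP_Interact is an interactable sign actor that shows a widget on approach and toggles sign text on the Interact input.
; It enables input from player controller 0 at BeginPlay.
; Sphere overlap events show and hide the widget without filtering the overlapping actor.
; Interact presses alternately show and hide SignText through a FlipFlop, gated by PlayerInRange, which these graphs never set.
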(event `self.ReceiveBeginPlay`
  (`self.EnableInput` (`GameplayStatics.GetPlayerController` 0)))

(event `self.Sphere.OnComponentBeginOverlap`
  (params (OverlappedComponent :type "PrimitiveComponent Object Reference") (OtherActor :type "Actor Object Reference") (OtherComp :type "PrimitiveComponent Object Reference") (OtherBodyIndex :type Integer) (bFromSweep :type Boolean) (SweepResult :type "HitResult Structure (by ref)"))
  (`SceneComponent.SetVisibility` (`self.Widget`) true false))

(event `self.Sphere.OnComponentEndOverlap`
  (params (OverlappedComponent :type "PrimitiveComponent Object Reference") (OtherActor :type "Actor Object Reference") (OtherComp :type "PrimitiveComponent Object Reference") (OtherBodyIndex :type Integer))
  (`SceneComponent.SetVisibility` (`self.Widget`) false false))

(event `InputAction|Interact`
  (params (Key :type "Key Structure"))
  (bind _signtext (`self.SignText`))
  (:`Pressed`
    (if (`self.bPlayerInRange`)
      (`/Engine/EditorBlueprintResources/StandardMacros.FlipFlop`
        (:`A`
          (`SceneComponent.SetVisibility` _signtext true false))
        (:`B`
          (`SceneComponent.SetVisibility` _signtext false false))))))

(fn `UserConstructionScript`)